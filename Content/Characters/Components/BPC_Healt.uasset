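; BPC_Healt is a character health component that tracks current health against a maximum and exposes getters for the value and its percentage.
; It fills health on BeginPlay through Recovery, and AddHealth caps healing at the maximum.
; Damage clamps health at zero and fires the EDDead dispatcher once through a DoOnce.
; The EDChange dispatcher fires on BeginPlay and healing, but not on damage.
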(event `self.ReceiveBeginPlay`
  (`self.Recovery`)
  (`self.ED_Change`))

(fn `AddHealth`
  (params (Add :type "Float (double-precision)"))
  (set `self.Healt` (`KismetMathLibrary.FMin` (+ Add (`self.Healt`)) (`self.MaxHealt`)))
  (`self.ED_Change`))

(fn `Damage`
  (params (Damage :type "Float (double-precision)"))
  (bind _output_get (set `self.Healt` (`KismetMathLibrary.FMax` (- (`self.Healt`) (`local.Damage`)))))
  (if (== _output_get 0.0)
    (`/Engine/EditorBlueprintResources/StandardMacros.DoOnce` false
      (:`Completed`
        (`self.ED_Dead`)))))

(fn `GetHealth`
  (returns (Healt :type "Float (double-precision)"))
  (return (`self.Healt`)))

(fn `GetPercentHealth`
  (returns (ReturnValue :type "Float (double-precision)"))
  (return (/ (`self.Healt`) (`self.MaxHealt`))))

(fn `Recovery`
  (set `self.Healt` (`self.MaxHealt`)))